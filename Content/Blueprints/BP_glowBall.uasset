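; BP_glowBall is a glowing physics ball that changes to a random color, gets pushed and plays a sound when a Player-tagged actor hits it.
; The push is an impulse along the hit normal.
; The construction script creates a dynamic Glow material and randomizes the starting color unless MyGameInstance's LoadGame flag is set.
; SetColor stores CurrentColor and applies it to the material and point light.
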(event `self.ReceiveBeginPlay`)

(event `self.StaticMeshComponent.OnComponentHit`
  (params (HitComponent :type "PrimitiveComponent Object Reference") (OtherActor :type "Actor Object Reference") (OtherComp :type "PrimitiveComponent Object Reference") (NormalImpulse :type "Vector Structure") (Hit :type "HitResult Structure (by ref)"))
  (if (`self.ActorHasTag` OtherActor "Player")
    (`self.SetRandomColor`)
    (`self.AddImpulse` Hit)
    (`GameplayStatics.PlaySoundAtLocation` (`self.HitSound`) (`.ImpactPoint` (`GameplayStatics.BreakHitResult` Hit)))))

(fn `AddImpulse`
  (params (Hit :type "HitResult Structure (by ref)"))
  (`PrimitiveComponent.AddImpulse` (`self.StaticMeshComponent`) (* (`.ImpactNormal` (`GameplayStatics.BreakHitResult` Hit)) 200000) "None" false))

(fn `SetColor`
  (params (Color :type "LinearColor Structure"))
  (bind _dynamicmaterial (`self.DynamicMaterial`))
  (set `self.CurrentColor` Color)
  (`MaterialInstanceDynamic.SetVectorParameterValue` _dynamicmaterial "Glow_Color" Color)
  (`MaterialInstanceDynamic.SetVectorParameterValue` _dynamicmaterial "Base_Color" Color)
  (`LightComponent.SetLightColor` (`self.PointLight`) Color true))

(fn `SetRandomColor`
  (`self.SetColor` (make `LinearColor` (`KismetMathLibrary.RandomFloatInRange` 0.0 1.0) (`KismetMathLibrary.RandomFloatInRange` 0.0 1.0) (`KismetMathLibrary.RandomFloatInRange` 0.0 1.0) 1.0)))

(fn `UserConstructionScript`
  (bind _returnvalue (`PrimitiveComponent.CreateDynamicMaterialInstance` (`self.StaticMeshComponent`) 0 "/Game/Materials/glow.glow"))
  (set `self.DynamicMaterial` _returnvalue)
  (bind _asmy_game_instance (cast `/Game/MyGameInstance` (`GameplayStatics.GetGameInstance`)))
  (if (not (`/Game/MyGameInstance.LoadGame` _asmy_game_instance))
    (`self.SetRandomColor`)))